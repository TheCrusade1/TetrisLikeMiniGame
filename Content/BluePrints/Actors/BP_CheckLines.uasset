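; BP_CheckLines is a Tetris-style line-clear manager that also owns the score and level UI.
; CheckLines adds 10 points, then finds rows where a box component overlaps ten BP_SingleBlock actors.
; Each full row increases DropAmount; those below CutOffLineZ lower it, award 100 points, advance the level counter and destroy their blocks with particles.
; Finally, blocks above the cutoff have TargetZ reduced by DropAmount.
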(event `self.ReceiveBeginPlay`
  (bind _returnvalue (`|CreateWidget` "/Game/BluePrints/Widgets/BP_UserWidget.BP_UserWidget_C"))
  (bind _output_get (set `self.UI` _returnvalue))
  (`UserWidget.AddToViewport` _output_get 0))

(event `Add100`
  (params (`Point Value` :type Integer))
  (bind _output_get (set `self.Points` (+ 100 `Point Value`)))
  (`/Game/BluePrints/Widgets/BP_UserWidget.UpdateScore` (`self.UI`) _output_get))

(event `Add 10`
  (params (`Point Value` :type Integer))
  (bind _output_get (set `self.Points` (+ 10 `Point Value`)))
  (`/Game/BluePrints/Widgets/BP_UserWidget.UpdateScore` (`self.UI`) _output_get))

(event `Add 1 Level`
  (params (`Level Value` :type Integer) (`Level Counter Value` :type Integer))
  (if (>= `Level Counter Value` 10)
    (set `self.LevelCounter` 1)
    (bind _output_get (set `self.LevelNumber` (+ 1 `Level Value`)))
    (else
      (set `self.LevelCounter` (+ 1 `Level Counter Value`))))
  (`/Game/BluePrints/Widgets/BP_UserWidget.UpdateLevel` (`self.UI`) _output_get))

(fn `CheckLines`
  (locals (`Overlapping Actors` :type "Array of Actor Object Reference") (DropAmount :type "Float (double-precision)") (CutOffLineZ :type "Float (double-precision)" :default 6000.0))
  (`self.Add 10` (`self.Points`))
  (for _array_element (`self.K2_GetComponentsByClass` "/Script/Engine.BoxComponent")
    (set `local.Overlapping Actors` (`PrimitiveComponent.GetOverlappingActors` _array_element "/Game/BluePrints/Actors/BP_SingleBlock.BP_SingleBlock_C"))
    (if (== (`KismetArrayLibrary.Array_Length` (`local.Overlapping Actors`)) 10)
      (set `local.DropAmount` (+ (`local.DropAmount`) 50.0))
      (bind (_returnvalue_x _returnvalue_y _returnvalue_z) (`KismetMathLibrary.BreakVector` (`SceneComponent.K2_GetComponentLocation` _array_element)))
      (if (< _returnvalue_z (`local.CutOffLineZ`))
        (set `local.CutOffLineZ` _returnvalue_z)
        (`self.Add100` (`self.Points`))
        (`self.Add 1 Level` (`self.LevelNumber`) (`self.LevelCounter`))
        (for _array_element_2 (`local.Overlapping Actors`)
          (`GameplayStatics.SpawnEmitterAtLocation` null (`self.K2_GetActorLocation` _array_element_2))
          (`self.K2_DestroyActor` _array_element_2)))))
  (bind _outactors (`GameplayStatics.GetAllActorsOfClass` "/Game/BluePrints/Actors/BP_SingleBlock.BP_SingleBlock_C"))
  (for _array_element_3 _outactors
    (bind (_returnvalue_x_2 _returnvalue_y_2 _returnvalue_z_2) (`KismetMathLibrary.BreakVector` (`self.K2_GetActorLocation` _array_element_3)))
    (if (> _returnvalue_z_2 (`local.CutOffLineZ`))
      (set `/Game/BluePrints/Actors/BP_SingleBlock.TargetZ` (- (`/Game/BluePrints/Actors/BP_SingleBlock.TargetZ` _array_element_3) (`local.DropAmount`)) _array_element_3))))

(fn `UserConstructionScript`)