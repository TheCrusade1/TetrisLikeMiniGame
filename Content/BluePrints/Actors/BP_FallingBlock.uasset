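; Player-controlled falling Tetris piece, built at construction as one of seven random four-cube shapes with a glow colour.
; A looping timer steps it down using line traces; Enhanced Input moves or rotates it, reverting on overlap, and speeds descent through global time dilation.
; On landing it spawns BP_SingleBlock at each cube, has CheckLinesActor check lines, spawns the next piece and destroys itself.
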(event `Add 10`
  (params (`Point Value` :type Integer))
  (bind _output_get (set `self.Points` (+ 10 `Point Value`)))
  (`/Game/BluePrints/Widgets/BP_UserWidget.UpdateScore` (`self.BP_Widget`) _output_get))

(event `self.ReceiveBeginPlay`
  (`self.EnableInputEnhanced`)
  (bind _returnvalue (`KismetSystemLibrary.K2_SetTimerDelegate` (delegate `DropBlock`) (`self.DropSpeed`) true))
  (set `self.BlockDroppingTimer` _returnvalue))

(event `RotateBlock`
  (`self.RotateFunction` :!label _label))

(event `DropBlock`
  (`self.DropFunction`))

(event `EnhancedInput|/Game/Inputs/IA_RotateBlock`
  (params (ActionValue :type Boolean) (ElapsedSeconds :type "Float (double-precision)") (TriggeredSeconds :type "Float (double-precision)") (InputAction :type "InputAction Object Reference" :default "/Game/Inputs/IA_RotateBlock.IA_RotateBlock"))
  (:`Started`
    (goto _label)))

(event `LeftBlock`
  (`self.Try Lateral Movement` 50.0 :!label _label_2))

(event `EnhancedInput|/Game/Inputs/IA_MoveBlockLeft`
  (params (ActionValue :type Boolean) (ElapsedSeconds :type "Float (double-precision)") (TriggeredSeconds :type "Float (double-precision)") (InputAction :type "InputAction Object Reference" :default "/Game/Inputs/IA_MoveBlockLeft.IA_MoveBlockLeft"))
  (:`Started`
    (goto _label_2)))

(event `RightBlock`
  (`self.Try Lateral Movement` -50.0 :!label _label_3))

(event `EnhancedInput|/Game/Inputs/IA_MoveBlockRight`
  (params (ActionValue :type Boolean) (ElapsedSeconds :type "Float (double-precision)") (TriggeredSeconds :type "Float (double-precision)") (InputAction :type "InputAction Object Reference" :default "/Game/Inputs/IA_MoveBlockRight.IA_MoveBlockRight"))
  (:`Started`
    (goto _label_3)))

(event `EnhancedInput|/Game/Inputs/IA_SpeedBlockDecend`
  (params (ActionValue :type Boolean) (ElapsedSeconds :type "Float (double-precision)") (TriggeredSeconds :type "Float (double-precision)") (InputAction :type "InputAction Object Reference" :default "/Game/Inputs/IA_SpeedBlockDecend.IA_SpeedBlockDecend"))
  (:`Started`
    (`GameplayStatics.SetGlobalTimeDilation` 5.0))
  (:`Completed`
    (`GameplayStatics.SetGlobalTimeDilation` 1.0)))

(fn `DropFunction`
  (bind _checklinesactor (`self.CheckLinesActor`))
  (set `self.ShouldDrop?` true)
  (for _array_element (`SceneComponent.GetChildrenComponents` (`self.DefaultSceneRoot`) false)
    (bind _returnvalue (`SceneComponent.K2_GetComponentLocation` _array_element))
    (bind (_outhit _returnvalue_2) (`KismetSystemLibrary.LineTraceSingleForObjects` _returnvalue (- _returnvalue (0.0 0.0 50.0)) (`|MakeArray` "ObjectTypeQuery1" :!type "EObjectTypeQuery Enum")))
    (if _returnvalue_2
      (`/Engine/EditorBlueprintResources/StandardMacros.DoOnce` false
        (:`Completed`
          (set `self.ShouldDrop?` false)
          (`KismetSystemLibrary.K2_ClearAndInvalidateTimerHandle` (`self.BlockDroppingTimer`))))))
  (if (`self.ShouldDrop?`)
    (`self.K2_AddActorWorldOffset` (0.0 0.0 -50.0))
    (else
      (for _array_element_2 (`SceneComponent.GetChildrenComponents` (`self.DefaultSceneRoot`) false)
        (`|SpawnActorFromClass` "/Game/BluePrints/Actors/BP_SingleBlock.BP_SingleBlock_C" (`KismetMathLibrary.MakeTransform` (`SceneComponent.K2_GetComponentLocation` _array_element_2)) "Undefined" "MultiplyWithRoot" null (`self.BlockColor`) null))
      (`/Game/BluePrints/Actors/BP_CheckLines.CheckLines` _checklinesactor)
      (`|SpawnActorFromClass` "BP_FallingBlock_C" (`KismetMathLibrary.MakeTransform` (0.0 -65.0 1000.0)) "Undefined" "MultiplyWithRoot" null _checklinesactor null)
      (`self.K2_DestroyActor`))))

(fn `EnableInputEnhanced`
  (`EnhancedInputSubsystemInterface.AddMappingContext` (pcsubsystem `EnhancedInputLocalPlayerSubsystem` (`GameplayStatics.GetPlayerController` 0)) "/Game/Inputs/IMC_InputMappingContext.IMC_InputMappingContext" 0 (struct))
  (`self.EnableInput` (`GameplayStatics.GetPlayerController` 0)))

(fn `make l block`
  ;[1 1 1] make l block
  (`StaticMeshComponent.SetStaticMesh` (`self.Cube1`) "/Game/Meshes/LBlockMesh/1_Lblock.1_Lblock")
  (`SceneComponent.K2_AddLocalOffset` (`self.Cube1`) (0.0 0.0 0.0) false false)
  (`StaticMeshComponent.SetStaticMesh` (`self.Cube2`) "/Game/Meshes/LBlockMesh/2_Lblock.2_Lblock")
  (`SceneComponent.K2_AddLocalOffset` (`self.Cube2`) (0.0 -50.0 0.0) false false)
  (`StaticMeshComponent.SetStaticMesh` (`self.Cube3`) "/Game/Meshes/LBlockMesh/3_Lblock.3_Lblock")
  (`SceneComponent.K2_AddLocalOffset` (`self.Cube3`) (0.0 0.0 50.0) false false)
  (`StaticMeshComponent.SetStaticMesh` (`self.Cube4`) "/Game/Meshes/LBlockMesh/4_Lblock.4_Lblock")
  (`SceneComponent.K2_AddLocalOffset` (`self.Cube4`) (0.0 0.0 100.0) false false))

(fn `make l R block`
  ;[1 1 1] make reverse l block
  (`StaticMeshComponent.SetStaticMesh` (`self.Cube1`) "/Game/Meshes/ReverseLBlockMesh/1_RLblock.1_RLblock")
  (`SceneComponent.K2_AddLocalOffset` (`self.Cube1`) (0.0 0.0 0.0) false false)
  (`StaticMeshComponent.SetStaticMesh` (`self.Cube2`) "/Game/Meshes/ReverseLBlockMesh/2_RLblock.2_RLblock")
  (`SceneComponent.K2_AddLocalOffset` (`self.Cube2`) (0.0 50.0 0.0) false false)
  (`StaticMeshComponent.SetStaticMesh` (`self.Cube3`) "/Game/Meshes/ReverseLBlockMesh/3_RLblock.3_RLblock")
  (`SceneComponent.K2_AddLocalOffset` (`self.Cube3`) (0.0 0.0 50.0) false false)
  (`StaticMeshComponent.SetStaticMesh` (`self.Cube4`) "/Game/Meshes/ReverseLBlockMesh/4_RLblock.4_RLblock")
  (`SceneComponent.K2_AddLocalOffset` (`self.Cube4`) (0.0 0.0 100.0) false false))

(fn `make line block`
  ;[1 1 1] make line block
  (`StaticMeshComponent.SetStaticMesh` (`self.Cube1`) "/Game/Meshes/LineBlockMesh/1_Line.1_Line")
  (`SceneComponent.K2_AddLocalOffset` (`self.Cube1`) (0.0 0.0 0.0) false false)
  (`StaticMeshComponent.SetStaticMesh` (`self.Cube2`) "/Game/Meshes/LineBlockMesh/2_Line.2_Line")
  (`SceneComponent.K2_AddLocalOffset` (`self.Cube2`) (0.0 0.0 50.0) false false)
  (`StaticMeshComponent.SetStaticMesh` (`self.Cube3`) "/Game/Meshes/LineBlockMesh/3_Line.3_Line")
  (`SceneComponent.K2_AddLocalOffset` (`self.Cube3`) (0.0 0.0 100.0) false false)
  (`StaticMeshComponent.SetStaticMesh` (`self.Cube4`) "/Game/Meshes/LineBlockMesh/4_Line.4_Line")
  (`SceneComponent.K2_AddLocalOffset` (`self.Cube4`) (0.0 0.0 150.0) false false))

(fn `make reverse s block`
  ;[1 1 1] make reverse s block
  (`StaticMeshComponent.SetStaticMesh` (`self.Cube1`) "/Game/Meshes/ReverseSBlock/1_RSblock.1_RSblock")
  (`SceneComponent.K2_AddLocalOffset` (`self.Cube1`) (0.0 0.0 0.0) false false)
  (`StaticMeshComponent.SetStaticMesh` (`self.Cube2`) "/Game/Meshes/ReverseSBlock/2_RSblock.2_RSblock")
  (`SceneComponent.K2_AddLocalOffset` (`self.Cube2`) (0.0 0.0 50.0) false false)
  (`StaticMeshComponent.SetStaticMesh` (`self.Cube3`) "/Game/Meshes/ReverseSBlock/3_RSblock.3_RSblock")
  (`SceneComponent.K2_AddLocalOffset` (`self.Cube3`) (0.0 -50.0 50.0) false false)
  (`StaticMeshComponent.SetStaticMesh` (`self.Cube4`) "/Game/Meshes/ReverseSBlock/4_RSblock.4_RSblock")
  (`SceneComponent.K2_AddLocalOffset` (`self.Cube4`) (0.0 -50.0 100.0) false false)
  (set `self.BlockColor` (struct :`G` 0.064577 :`B` 1.0 :`A` 1.0)))

(fn `make s block`
  (`StaticMeshComponent.SetStaticMesh` (`self.Cube1`) "/Game/Meshes/SBlockMesh/1_Sblock.1_Sblock")
  ;[1 1 1] make s block
  (`SceneComponent.K2_AddLocalOffset` (`self.Cube1`) (0.0 0.0 0.0) false false)
  (`StaticMeshComponent.SetStaticMesh` (`self.Cube2`) "/Game/Meshes/SBlockMesh/2_Sblock.2_Sblock")
  (`SceneComponent.K2_AddLocalOffset` (`self.Cube2`) (0.0 0.0 50.0) false false)
  (`StaticMeshComponent.SetStaticMesh` (`self.Cube3`) "/Game/Meshes/SBlockMesh/3_Sblock.3_Sblock")
  (`SceneComponent.K2_AddLocalOffset` (`self.Cube3`) (0.0 50.0 50.0) false false)
  (`StaticMeshComponent.SetStaticMesh` (`self.Cube4`) "/Game/Meshes/SBlockMesh/4_Sblock.4_Sblock")
  (`SceneComponent.K2_AddLocalOffset` (`self.Cube4`) (0.0 50.0 100.0) false false)
  (set `self.BlockColor` (struct :`R` 1.0 :`B` 0.715499 :`A` 1.0)))

(fn `make square block`
  ;[1 1 1] make square block
  (`StaticMeshComponent.SetStaticMesh` (`self.Cube1`) "/Game/Meshes/CubeBlockMesh/1_CubeBlock.1_CubeBlock")
  (`SceneComponent.K2_AddLocalOffset` (`self.Cube1`) (0.0 50.0 0.0) false false)
  (`StaticMeshComponent.SetStaticMesh` (`self.Cube2`) "/Game/Meshes/CubeBlockMesh/2_CubeBlock.2_CubeBlock")
  (`SceneComponent.K2_AddLocalOffset` (`self.Cube2`) (0.0 0.0 0.0) false false)
  (`StaticMeshComponent.SetStaticMesh` (`self.Cube3`) "/Game/Meshes/CubeBlockMesh/3_CubeBlock.3_CubeBlock")
  (`SceneComponent.K2_AddLocalOffset` (`self.Cube3`) (0.0 50.0 50.0) false false)
  (`StaticMeshComponent.SetStaticMesh` (`self.Cube4`) "/Game/Meshes/CubeBlockMesh/4_CubeBlock.4_CubeBlock")
  (`SceneComponent.K2_AddLocalOffset` (`self.Cube4`) (0.0 0.0 50.0) false false))

(fn `make t block`
  ;[1 1 1] make t block
  (`StaticMeshComponent.SetStaticMesh` (`self.Cube1`) "/Game/Meshes/TBlockMesh/1_Tblock.1_Tblock")
  (`SceneComponent.K2_AddLocalOffset` (`self.Cube1`) (0.0 50.0 0.0) false false)
  (`StaticMeshComponent.SetStaticMesh` (`self.Cube2`) "/Game/Meshes/TBlockMesh/2_Tblock.2_Tblock")
  (`SceneComponent.K2_AddLocalOffset` (`self.Cube2`) (0.0 0.0 0.0) false false)
  (`SceneComponent.K2_AddLocalOffset` (`self.Cube2`) (0.0 0.0 0.0) false false)
  (`StaticMeshComponent.SetStaticMesh` (`self.Cube3`) "/Game/Meshes/TBlockMesh/3_Tblock.3_Tblock")
  (`SceneComponent.K2_AddLocalOffset` (`self.Cube3`) (0.0 0.0 25.0) false false)
  (`SceneComponent.K2_AddLocalOffset` (`self.Cube3`) (0.0 0.0 25.0) false false)
  (`StaticMeshComponent.SetStaticMesh` (`self.Cube4`) "/Game/Meshes/TBlockMesh/4_Tblock.4_Tblock")
  (`SceneComponent.K2_AddLocalOffset` (`self.Cube4`) (0.0 -25.0 0.0) false false)
  (`SceneComponent.K2_AddLocalOffset` (`self.Cube4`) (0.0 -25.0 0.0) false false))

(fn `RotateFunction`
  (`self.K2_AddActorLocalRotation` (struct :`Roll` 90.0))
  (for _array_element (`self.K2_GetComponentsByClass` "/Script/Engine.StaticMeshComponent")
    (bind (_outactors _returnvalue) (`KismetSystemLibrary.BoxOverlapActors` (`SceneComponent.K2_GetComponentLocation` _array_element) (15.0 0.0 0.0) (`|MakeArray` "ObjectTypeQuery1" :!type "EObjectTypeQuery Enum")))
    (if _returnvalue
      (`self.K2_AddActorLocalRotation` (struct :`Roll` -90.0))
      (break))))

(fn `Try Lateral Movement`
  (params (MoveAmount :type "Float (double-precision)"))
  (`self.K2_AddActorWorldOffset` (`KismetMathLibrary.MakeVector` 0.0 MoveAmount))
  (for _array_element (`self.K2_GetComponentsByClass` "/Script/Engine.StaticMeshComponent")
    (bind (_outactors _returnvalue) (`KismetSystemLibrary.BoxOverlapActors` (`SceneComponent.K2_GetComponentLocation` _array_element) (15.0 0.0 0.0) (`|MakeArray` "ObjectTypeQuery1" :!type "EObjectTypeQuery Enum")))
    (if _returnvalue
      (`self.K2_AddActorWorldOffset` (`KismetMathLibrary.MakeVector` 0.0 (* MoveAmount -1.0)))
      (break))))

(fn `UserConstructionScript`
  (switch `int` (`KismetMathLibrary.RandomIntegerInRange` 0 6)
    (:`0`
      (`self.make line block`))
    (:`1`
      (`self.make l block`))
    (:`2`
      (`self.make l R block`))
    (:`3`
      (`self.make s block`))
    (:`4`
      (`self.make reverse s block`))
    (:`5`
      (`self.make t block`))
    (:`6`
      (`self.make square block`)))
  (`MeshComponent.SetVectorParameterValueOnMaterials` (`self.Cube1`) "GlowColor" (`KismetMathLibrary.Conv_LinearColorToVector` (`self.BlockColor`)))
  (`MeshComponent.SetVectorParameterValueOnMaterials` (`self.Cube2`) "GlowColor" (`KismetMathLibrary.Conv_LinearColorToVector` (`self.BlockColor`)))
  (`MeshComponent.SetVectorParameterValueOnMaterials` (`self.Cube3`) "GlowColor" (`KismetMathLibrary.Conv_LinearColorToVector` (`self.BlockColor`)))
  (`MeshComponent.SetVectorParameterValueOnMaterials` (`self.Cube4`) "GlowColor" (`KismetMathLibrary.Conv_LinearColorToVector` (`self.BlockColor`))))